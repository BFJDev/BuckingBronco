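; Level 3 objective Blueprint that scores a point when a Cube actor enters its Box trigger.
; On overlap it destroys the cube, prints a score message and increments the Score stored on the player's Bronco5 pawn.
; When Score exactly equals ScoreToWin from the BroncoGame game mode, it opens the Main level.
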(event OnComponentBeginOverlap(Box)
  (params (OverlappedComponent :type Primitive%20Component%20Object%20Reference) (OtherActor :type Actor%20Object%20Reference) (OtherComp :type Primitive%20Component%20Object%20Reference) (OtherBodyIndex :type Integer) (bFromSweep :type Boolean) (SweepResult :type Hit%20Result%20Structure%20%28by%20ref%29))
  (bind _ascube (Utilities|Casting|CastToCube OtherActor))
  (Actor|DestroyActor _ascube)
  (Development|PrintString "Score!!!!!" true true "(R=0.809878,G=0.082176,B=1.000000,A=1.000000)")
  (bind _asbronco_5 (Utilities|Casting|CastToBronco5 (Game|Player|GetPlayerPawn 0)))
  (bind _output_get (Variables|/Game/MyContent/Blueprints/Bronco5.Bronco5_C|SetScore _asbronco_5 (+ (Variables|/Game/MyContent/Blueprints/Bronco5.Bronco5_C|GetScore _asbronco_5) 1.0)))
  (bind _asbronco_game (Utilities|Casting|CastToBroncoGame (Game|GetGameMode)))
  (if (== _output_get (Variables|/Game/MyContent/Blueprints/BroncoGame.BroncoGame_C|GetScoreToWin _asbronco_game))
    (Game|OpenLevel(byName) "Main")))

(fn ConstructionScript)