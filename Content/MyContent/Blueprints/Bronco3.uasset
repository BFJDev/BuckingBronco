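; Player-controlled Bronco Blueprint: a drivable body with a bucking arm.
; Axis inputs move and turn the actor by local offsets, a camera action yaws the spring arm, and M opens the pause menu without pausing the game.
; Buck, gated by IsBucking, kicks the arm up, then lowers it after a delay via a ForLoopWithDelay macro.
; Arm hit and end-overlap events with Cubes toggle CanBuckCube; HUD creation is unwired.
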(event OnComponentEndOverlap(Bronco_Arm_2)
  (params (OverlappedComponent :type Primitive%20Component%20Object%20Reference) (OtherActor :type Actor%20Object%20Reference) (OtherComp :type Primitive%20Component%20Object%20Reference) (OtherBodyIndex :type Integer))
  (Utilities|Casting|CastToCube OtherActor)
  (Variables|Default|SetCan%20Buck%20Cube false))

(event OnComponentHit(Bronco_Arm_2)
  (params (HitComponent :type Primitive%20Component%20Object%20Reference) (OtherActor :type Actor%20Object%20Reference) (OtherComp :type Primitive%20Component%20Object%20Reference) (NormalImpulse :type Vector :default "0, 0, 0") (Hit :type Hit%20Result%20Structure%20%28by%20ref%29))
  (Utilities|Casting|CastToCube OtherActor)
  (Variables|Default|SetCan%20Buck%20Cube true))

(event EventBeginPlay)

(event Input|ActionEvents|InputActionBuck
  (params (Key :type Key%20Structure))
  (:Pressed
    (Physics|AddImpulseatLocation (Variables|Default|GetBronco_Body_Complete_2) "0, 0, 0" "100.000000, 0, 0" "None")
    ;[1 1 1] Bucking Action
    (if (not (Variables|Default|GetIs%20Bucking))
      (Variables|Default|SetIs%20Bucking true)
      (Class|PrimitiveComponent|AddAngularImpulseinDegrees (Variables|Default|GetBronco_Arm_2) "0.000000,200.000000,200.000000" "None" false)
      (for _index (range 0 20)
        (Transformation|AddLocalRotation (Variables|Default|GetBronco_Arm_2) (Math|Rotator|MakeRotator 0.0 1.0 0.0) false false))
      (Utilities|FlowControl|Delay 2.0)
      (Utilities|ForLoopwithDelay 0 20 0.002
        (:loop%20body
          (Transformation|AddLocalRotation (Variables|Default|GetBronco_Arm_2) (Math|Rotator|MakeRotator 0.0 -1.0 0.0) false false))
        (:completed
          (Variables|Default|SetIs%20Bucking false))))))

(event Input|ActionEvents|InputActionChangeCamera
  (params (Key :type Key%20Structure))
  ;[1 1 1] Change Camera view
  (:Pressed
    (Transformation|AddRelativeRotation (Variables|Default|GetSpringArm) (Math|Rotator|MakeRotator 0.0 0.0 (Variables|Default|GetCamera%20Angle%20Change)) false false)))

(event Input|AxisEvents|InputAxisMoveForward
  (params (AxisValue :type Float%20%28single-precision%29))
  ;[1 1 1] Forward Movement
  (Transformation|AddActorLocalOffset (Math|Vector|MakeVector (* AxisValue (Variables|Default|GetForward%20Speed)) 0.0 0.0) false false))

(event Input|AxisEvents|InputAxisMoveRight
  (params (AxisValue :type Float%20%28single-precision%29))
  ;[1 1 1] Right Turn
  (Transformation|AddActorLocalRotation (Math|Rotator|MakeRotator 0.0 0.0 (* AxisValue (Variables|Default|GetTurning%20Speed))) false false))

(event Input|KeyboardEvents|M
  (params (Key :type Key%20Structure))
  (bind _returnvalue (Game|GetPlayerController 0))
  (:Pressed
    (Utilities|IsValid (Variables|Default|GetPause%20Menu%20Reference)
      (:Is%20Valid
        _)
      (:Is%20Not%20Valid
        (bind _returnvalue_2 (UserInterface|CreateWidget "/Game/MyContent/Blueprints/Menus+HUDs/Pause_Menu.Pause_Menu_C"))
        (Variables|Default|SetPause%20Menu%20Reference _returnvalue_2)))
    (Variables|/Script/Engine.PlayerController|SetbShowMouseCursor _returnvalue true)
    (Input|SetInputModeUIOnly _returnvalue (Variables|Default|GetPause%20Menu%20Reference) "DoNotLock")
    (UserInterface|Viewport|AddtoViewport (Variables|Default|GetPause%20Menu%20Reference) 0)
    (Game|SetGamePaused false)))

(fn ConstructionScript)