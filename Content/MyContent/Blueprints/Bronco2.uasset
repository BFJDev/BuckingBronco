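; Bronco2 is a player-controlled Blueprint actor that drives, turns and performs a bucking arm action.
; Axis inputs apply local offset and yaw each frame, scaled by speed variables but not delta time.
; ChangeCamera steps the spring arm's yaw by a set angle per press.
; Buck raises and tilts BroncoArm, holds it through a Delay, then reverses both transforms, with CanBuck blocking re-triggering until done.
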(event Input|ActionEvents|InputActionBuck
  (params (Key :type Key%20Structure))
  (bind _bronco_arm (Variables|Default|GetBronco_Arm))
  (bind _bronco_arm_2 (Variables|Default|GetBronco_Arm))
  ;[1 1 1] Bucking Action
  (:Pressed
    (if (Variables|Default|GetCan%20Buck)
      (Variables|Default|SetCan%20Buck false) ; On button press, prevent further input until action is complete
      (Transformation|AddLocalOffset _bronco_arm (Math|Vector|MakeVector 0.0 0.0 (Variables|Default|GetBuck%20Forward)) false false) ; Move the Arm slightly up
      (Transformation|AddLocalRotation _bronco_arm (Math|Rotator|MakeRotator 0.0 (Variables|Default|GetBuck_Up) 0.0) false false) ; Rotate the Arm slightly up
      (Utilities|FlowControl|Delay (Variables|Default|GetDelay%20Time)) ; Pause the action for a moment, holding the arm up
      (Transformation|AddLocalRotation _bronco_arm_2 (Math|Rotator|MakeRotator 0.0 (- 0.0 (Variables|Default|GetBuck_Up)) 0.0) false false) ; Return the Arm to resting position
      (Transformation|AddLocalOffset _bronco_arm_2 (Math|Vector|MakeVector 0.0 0.0 (- 0.0 (Variables|Default|GetBuck%20Forward))) false false) ; Return the Arm to resting Place
      (Variables|Default|SetCan%20Buck true))))

(event Input|ActionEvents|InputActionChangeCamera
  (params (Key :type Key%20Structure))
  ;[1 1 1] Change Camera view
  (:Pressed
    (Transformation|AddRelativeRotation (Variables|Default|GetSpringArm) (Math|Rotator|MakeRotator 0.0 0.0 (Variables|Default|GetCamera%20Angle%20Change)) false false)))

(event Input|AxisEvents|InputAxisMoveForward
  (params (AxisValue :type Float%20%28single-precision%29))
  ;[1 1 1] Forward Movement
  (Transformation|AddActorLocalOffset (Math|Vector|MakeVector (* AxisValue (Variables|Default|GetForward%20Speed)) 0.0 0.0) false false))

(event Input|AxisEvents|InputAxisMoveRight
  (params (AxisValue :type Float%20%28single-precision%29))
  ;[1 1 1] Right Turn
  (Transformation|AddActorLocalRotation (Math|Rotator|MakeRotator 0.0 0.0 (* AxisValue (Variables|Default|GetTurning%20Speed))) false false))

(fn ConstructionScript)