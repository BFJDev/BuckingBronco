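; CubeB is a cube that gets launched when a Bronco5 flipping arm hits it.
; On Hit, it checks that the Bronco can buck cubes and is bucking, then applies impulses along the hit normal and upward, scaled by XPower and YPower.
; A Hit flag with a two-second delayed reset blocks repeat launches from continuous arm contact.
; An unconnected TestBronco version of the logic remains.
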(event Collision|EventHit
  (params (MyComp :type Primitive%20Component%20Object%20Reference) (Other :type Actor%20Object%20Reference) (OtherComp :type Primitive%20Component%20Object%20Reference) (bSelfMoved :type Boolean) (HitLocation :type Vector :default "0, 0, 0") (HitNormal :type Vector :default "0, 0, 0") (NormalImpulse :type Vector :default "0, 0, 0") (Hit :type Hit%20Result%20Structure%20%28by%20ref%29))
  (bind _cubemesh (Variables|Default|GetCubeMesh))
  ;[1 1 1] Make cast to Bronco
  (bind _asbronco_5 (Utilities|Casting|CastToBronco5 Other))
  ;[1 1 1] Check if Bronco has fired the flipping arm, and if this is the first hit (since continuous contact with arm after first hit can produce unwanted behavior)
  (if (Variables|/Game/MyContent/Blueprints/Bronco5.Bronco5_C|GetCan%20Buck%20Cube _asbronco_5)
    (if (Variables|/Game/MyContent/Blueprints/Bronco5.Bronco5_C|GetIs%20Bucking _asbronco_5)
      (if (not (Variables|Default|GetHit))
        (Variables|Default|SetHit true)
        (Development|PrintString "Hit")
        ;[1 1 1] Add the forward and upward impulse to launch the cube
        (Physics|AddImpulse _cubemesh (* HitNormal (Variables|/Game/MyContent/Blueprints/Bronco5.Bronco5_C|GetX_Power _asbronco_5)) "None" false)
        (Physics|AddImpulse _cubemesh (Math|Vector|MakeVector 0.0 0.0 (Variables|/Game/MyContent/Blueprints/Bronco5.Bronco5_C|GetY_Power _asbronco_5)) "None" false)
        ;[1 1 1] Reset "Hit" variable
        (Utilities|FlowControl|Delay 2.0)
        (Variables|Default|SetHit false)))))

(fn ConstructionScript)