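; Bronco4 is a player-driven Blueprint, apparently a vehicle, with simple movement and a switchable camera angle.
; MoveForward and MoveRight axis inputs apply local offset and yaw rotation each frame, scaled by ForwardSpeed and TurningSpeed, without delta-time scaling.
; Pressing ChangeCamera yaws the SpringArm by CameraAngleChange, stepping the view around the actor.
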(event Input|ActionEvents|InputActionChangeCamera
  (params (Key :type Key%20Structure))
  ;[1 1 1] Change Camera view
  (:Pressed
    (Transformation|AddRelativeRotation (Variables|Default|GetSpringArm) (Math|Rotator|MakeRotator 0.0 0.0 (Variables|Default|GetCamera%20Angle%20Change)) false false)))

(event Input|AxisEvents|InputAxisMoveForward
  (params (AxisValue :type Float%20%28single-precision%29))
  ;[1 1 1] Forward Movement
  (Transformation|AddActorLocalOffset (Math|Vector|MakeVector (* AxisValue (Variables|Default|GetForward%20Speed)) 0.0 0.0) false false))

(event Input|AxisEvents|InputAxisMoveRight
  (params (AxisValue :type Float%20%28single-precision%29))
  ;[1 1 1] Right Turn
  (Transformation|AddActorLocalRotation (Math|Rotator|MakeRotator 0.0 0.0 (* AxisValue (Variables|Default|GetTurning%20Speed))) false false))

(fn ConstructionScript)